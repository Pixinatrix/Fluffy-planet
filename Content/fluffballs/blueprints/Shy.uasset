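; Shy is a fleeing behavior that starts when Pawn Sensing sees or hears something.
; It flags SensingPlayer and calls ShyAway, which runs AI MoveTo on the Instigator and re-triggers itself on success or failure.
; The destination comes from a random navigable point node that never executes.
; That node's origin multiplies actor location by a reversed look-at vector toward CharacterRef, rather than adding an offset.
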(event OnHearNoise(PawnSensing)
  (params (Instigator :type Pawn%20Object%20Reference) (Location :type Vector%20%28by%20ref%29 :default "0, 0, 0") (Volume :type Float%20%28single-precision%29))
  (Variables|Default|Setsensing%20player true)
  (CallFunction|ShyAway))

(event OnSeePawn(PawnSensing)
  (params (Pawn :type Pawn%20Object%20Reference))
  (Variables|Default|Setsensing%20player true)
  (CallFunction|ShyAway))

(event Custom|Shy%20away
  (AI|AIMoveTo (Variables|Actor|GetInstigator) (stale _randomlocation) 0 5.0 false
    (:OnSuccess
      _)
    (:OnFail
      _))
  (CallFunction|ShyAway))

(event EventBeginPlay)

(event Collision|EventActorBeginOverlap
  (params (OtherActor :type Actor%20Object%20Reference)))

(event EventTick
  (params (DeltaSeconds :type Float%20%28single-precision%29)))

(fn ConstructionScript)